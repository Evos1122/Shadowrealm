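; BP_DamageVolume is a trigger volume that deals a fixed amount of damage to actors with a BP_HealthComponent when they begin overlapping it.
; BeginPlay configures DamageTrigger as a query-only overlap and disables collision on DamageVisual.
; DamageActor finds the health component on the overlapping actor and calls TakeDamage, ignoring actors without one.
; DamagePlayer and HealPlayer apply damage or healing directly to player 0, but nothing in this Blueprint calls them.
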(event `self.ReceiveBeginPlay`
  (`PrimitiveComponent.SetCollisionProfileName` (`self.DamageTrigger`) "OverlapAllDynamic" true)
  (`PrimitiveComponent.SetCollisionEnabled` (`self.DamageTrigger`) "QueryOnly")
  (set `PrimitiveComponent.bGenerateOverlapEvents` true (`self.DamageTrigger`))
  (`PrimitiveComponent.SetCollisionEnabled` (`self.DamageVisual`) "NoCollision"))

(event `self.DamageTrigger.OnComponentBeginOverlap`
  (params (OverlappedComponent :type "PrimitiveComponent Object Reference") (OtherActor :type "Actor Object Reference") (OtherComp :type "PrimitiveComponent Object Reference") (OtherBodyIndex :type Integer) (bFromSweep :type Boolean) (SweepResult :type "HitResult Structure (by ref)"))
  (`self.DamageActor` OtherActor))

(fn `DamageActor`
  (params (TargetActor :type "Actor Object Reference"))
  (bind _asbp_health_component (cast `/Game/Health/BP_HealthComponent` (`self.GetComponentByClass` TargetActor "/Game/Health/BP_HealthComponent.BP_HealthComponent_C")))
  (`/Game/Health/BP_HealthComponent.TakeDamage` _asbp_health_component 25.0))

(fn `DamagePlayer`
  (`self.DamageActor` self (`GameplayStatics.GetPlayerCharacter` 0)))

(fn `HealPlayer`
  (params (HealAmount :type "Float (double-precision)"))
  (bind _asbp_health_component (cast `/Game/Health/BP_HealthComponent` (`self.GetComponentByClass` (`GameplayStatics.GetPlayerCharacter` 0) "/Game/Health/BP_HealthComponent.BP_HealthComponent_C")))
  (`/Game/Health/BP_HealthComponent.Heal` _asbp_health_component HealAmount))

(fn `UserConstructionScript`)