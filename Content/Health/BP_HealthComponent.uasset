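; Health component that tracks an actor's current health against a maximum, starting full on BeginPlay.
; TakeDamage and Heal clamp health within that range, broadcast OnHealthChanged and print the new value, while IsDead reports zero health.
; A DeathBroadcast flag makes OnDeath fire, with a printed death message, only once until healing lifts health above zero again.
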(event `self.ReceiveBeginPlay`
  (set `self.CurrentHealth` (`self.MaxHealth`))
  (set `self.DeathBroadcast` false)
  (`self.OnHealthChanged` self (`self.CurrentHealth`) (`self.MaxHealth`)))

(fn `Heal`
  (params (HealAmount :type "Float (double-precision)"))
  (if (> HealAmount 0.0)
    (set `self.CurrentHealth` (`KismetMathLibrary.FClamp` (+ (`self.CurrentHealth`) HealAmount) 0.0 (`self.MaxHealth`)))
    (if (> (`self.CurrentHealth`) 0.0)
      (set `self.DeathBroadcast` false))
    (`self.OnHealthChanged` self (`self.CurrentHealth`) (`self.MaxHealth`))
    (`KismetSystemLibrary.PrintString` (`KismetStringLibrary.Conv_DoubleToString` (`self.CurrentHealth`)) true true (struct :`G` 0.66 :`B` 1.0 :`A` 1.0) 3.0)))

(fn `IsDead`
  (returns (Dead :type Boolean))
  (return (<= (`self.CurrentHealth`) 0.0)))

(fn `TakeDamage`
  (params (DamageAmount :type "Float (double-precision)"))
  (if (> DamageAmount 0.0)
    (set `self.CurrentHealth` (`KismetMathLibrary.FClamp` (- (`self.CurrentHealth`) DamageAmount) 0.0 (`self.MaxHealth`)))
    (`self.OnHealthChanged` self (`self.CurrentHealth`) (`self.MaxHealth`))
    (`KismetSystemLibrary.PrintString` (`KismetStringLibrary.Conv_DoubleToString` (`self.CurrentHealth`)) true true (struct :`G` 0.66 :`B` 1.0 :`A` 1.0) 3.0)
    (if (and (<= (`self.CurrentHealth`) 0.0) (not (`self.DeathBroadcast`)))
      (set `self.DeathBroadcast` true)
      (`self.OnDeath` self)
      (`KismetSystemLibrary.PrintString` (`self.DeathMessage`) true true (struct :`G` 0.66 :`B` 1.0 :`A` 1.0) 3.0))))