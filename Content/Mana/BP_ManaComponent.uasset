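; Mana component that tracks an actor's mana pool, starting full, with functions to spend, restore and check it, broadcasting changes through OnManaChanged.
; A successful spend restarts a delay timer, after which regeneration begins and repeats on a looping timer until mana is full.
; Regeneration requires a living BP_HealthComponent on the owner and clears its timers if that component is missing or reports death.
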(event `self.ReceiveBeginPlay`
  (set `self.CurrentMana` (`self.MaxMana`))
  (`self.OnManaChanged` self (`self.CurrentMana`) (`self.MaxMana`)))

(fn `BeginManaRegeneration`
  (bind _returnvalue (`self.GetOwner` self))
  (`/Engine/EditorBlueprintResources/StandardMacros.IsValid` _returnvalue
    (:`Is Valid`
      (bind _asbp_health_component (cast `/Game/Health/BP_HealthComponent` (`Actor.GetComponentByClass` _returnvalue "/Game/Health/BP_HealthComponent.BP_HealthComponent_C"))
        (:`then`
          (bind _dead (`/Game/Health/BP_HealthComponent.IsDead` _asbp_health_component))
          (if (and (not _dead) (< (`self.CurrentMana`) (`self.MaxMana`)))
            (`self.RestoreMana` self 5.0)
            (if (< (`self.CurrentMana`) (`self.MaxMana`))
              (`KismetSystemLibrary.K2_SetTimer` self "RegenerateMana" 1.0 true))
            (else
              (`KismetSystemLibrary.K2_ClearTimer` self "BeginManaRegeneration")
              (`KismetSystemLibrary.K2_ClearTimer` self "RegenerateMana"))))
        (:`CastFailed`
          (`KismetSystemLibrary.K2_ClearTimer` self "BeginManaRegeneration")
          (`KismetSystemLibrary.K2_ClearTimer` self "RegenerateMana"))))
    (:`Is Not Valid`
      (`KismetSystemLibrary.K2_ClearTimer` self "BeginManaRegeneration")
      (`KismetSystemLibrary.K2_ClearTimer` self "RegenerateMana"))))

(fn `HasEnoughMana`
  (params (ManaCost :type "Float (double-precision)"))
  (returns (ReturnValue :type Boolean))
  (return (and (>= ManaCost 0.0) (>= (`self.CurrentMana`) ManaCost))))

(fn `RegenerateMana`
  (bind _returnvalue (`self.GetOwner` self))
  (`/Engine/EditorBlueprintResources/StandardMacros.IsValid` _returnvalue
    (:`Is Valid`
      (bind _asbp_health_component (cast `/Game/Health/BP_HealthComponent` (`Actor.GetComponentByClass` _returnvalue "/Game/Health/BP_HealthComponent.BP_HealthComponent_C"))
        (:`then`
          (bind _dead (`/Game/Health/BP_HealthComponent.IsDead` _asbp_health_component))
          (if (and (not _dead) (< (`self.CurrentMana`) (`self.MaxMana`)))
            (`self.RestoreMana` self 5.0)
            (else
              (`KismetSystemLibrary.K2_ClearTimer` self "BeginManaRegeneration")
              (`KismetSystemLibrary.K2_ClearTimer` self "RegenerateMana"))))
        (:`CastFailed`
          (`KismetSystemLibrary.K2_ClearTimer` self "BeginManaRegeneration")
          (`KismetSystemLibrary.K2_ClearTimer` self "RegenerateMana"))))
    (:`Is Not Valid`
      (`KismetSystemLibrary.K2_ClearTimer` self "BeginManaRegeneration")
      (`KismetSystemLibrary.K2_ClearTimer` self "RegenerateMana"))))

(fn `RestoreMana`
  (params (ManaAmount :type "Float (double-precision)"))
  (if (> ManaAmount 0.0)
    (set `self.CurrentMana` (`KismetMathLibrary.FClamp` (+ (`self.CurrentMana`) ManaAmount) 0.0 (`self.MaxMana`)))
    (`self.OnManaChanged` self (`self.CurrentMana`) (`self.MaxMana`))
    (if (>= (`self.CurrentMana`) (`self.MaxMana`))
      (`KismetSystemLibrary.K2_ClearTimer` self "BeginManaRegeneration")
      (`KismetSystemLibrary.K2_ClearTimer` self "RegenerateMana"))))

(fn `SpendMana`
  (params (ManaCost :type "Float (double-precision)"))
  (returns (Success :type Boolean))
  (if (and (> ManaCost 0.0) (>= (`self.CurrentMana`) ManaCost))
    (set `self.CurrentMana` (`KismetMathLibrary.FClamp` (- (`self.CurrentMana`) ManaCost) 0.0 (`self.MaxMana`)))
    (`self.OnManaChanged` self (`self.CurrentMana`) (`self.MaxMana`))
    (`KismetSystemLibrary.K2_ClearTimer` self "BeginManaRegeneration")
    (`KismetSystemLibrary.K2_ClearTimer` self "RegenerateMana")
    (`KismetSystemLibrary.K2_SetTimer` self "BeginManaRegeneration" 2.0)
    (return true)
    (else
      (return false))))