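; BP_ShadowBurst is a short-lived magic area burst that damages nearby actors once and destroys itself after under a second.
; Shortly after BeginPlay, a one-shot timer applies fixed damage through BP_HealthComponent to actors overlapping CollisionSphere, excluding itself and its owner.
; A looping timer scales BoltVisual up and lowers its OpacityStrength material parameter in steps, then clears itself after a set step count.
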(event `self.ReceiveBeginPlay`
  (set `self.BurstVisualStep` 0.0)
  (`SceneComponent.SetRelativeScale3D` (`self.BoltVisual`) (`KismetMathLibrary.MakeVector` 0.45 0.45 0.45))
  (`MeshComponent.SetScalarParameterValueOnMaterials` (`self.BoltVisual`) "OpacityStrength" 0.32)
  (`KismetSystemLibrary.K2_SetTimer` self "ProcessBurst" 0.02 false false 0.0 0.0)
  (`KismetSystemLibrary.K2_SetTimer` self "UpdateBurstVisual" 0.05 true false 0.0 0.0)
  (`self.SetLifeSpan` self 0.75))

(fn `ProcessBurst`
  (for _array_element (`PrimitiveComponent.GetOverlappingActors` (`self.CollisionSphere`) "/Script/Engine.Actor")
    (if (and (!= _array_element self) (!= _array_element (`self.GetOwner` self)))
      (bind _returnvalue (`self.GetComponentByClass` _array_element "/Game/Health/BP_HealthComponent.BP_HealthComponent_C"))
      (`/Engine/EditorBlueprintResources/StandardMacros.IsValid` _returnvalue
        (:`Is Valid`
          (bind _asbp_health_component (cast `/Game/Health/BP_HealthComponent` _returnvalue))
          (`/Game/Health/BP_HealthComponent.TakeDamage` _asbp_health_component 25.0))))))

(fn `UpdateBurstVisual`
  (bind _returnvalue (+ (`self.BurstVisualStep`) 1.0))
  (bind _returnvalue_2 (+ 0.45 (* _returnvalue 0.16)))
  (set `self.BurstVisualStep` _returnvalue)
  (`SceneComponent.SetRelativeScale3D` (`self.BoltVisual`) (`KismetMathLibrary.MakeVector` _returnvalue_2 _returnvalue_2 _returnvalue_2))
  (`MeshComponent.SetScalarParameterValueOnMaterials` (`self.BoltVisual`) "OpacityStrength" (- 0.32 (* _returnvalue 0.03)))
  (if (>= _returnvalue 10.0)
    (`KismetSystemLibrary.K2_ClearTimer` self "UpdateBurstVisual")))

(fn `UserConstructionScript`)