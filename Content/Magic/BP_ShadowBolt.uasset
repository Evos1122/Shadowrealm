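; BP_ShadowBolt is a magic projectile actor that damages what its collision sphere overlaps.
; Each overlap calls ProcessImpact, which ignores itself, its owner and repeat impacts via the ImpactProcessed flag.
; A target with a BP_HealthComponent takes DamageAmount and the bolt destroys itself; other actors leave it intact.
; An unconnected copy of the impact logic, filtering by instigator instead of owner, never runs.
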(event `self.CollisionSphere.OnComponentBeginOverlap`
  (params (OverlappedComponent :type "PrimitiveComponent Object Reference") (OtherActor :type "Actor Object Reference") (OtherComp :type "PrimitiveComponent Object Reference") (OtherBodyIndex :type Integer) (bFromSweep :type Boolean) (SweepResult :type "HitResult Structure (by ref)"))
  (`self.ProcessImpact` OtherActor))

(fn `ProcessImpact`
  (params (OtherActor :type "Actor Object Reference"))
  (if (and (!= OtherActor self) (and (!= OtherActor (`self.GetOwner` self)) (not (`self.bImpactProcessed`))))
    (bind _asbp_health_component (cast `/Game/Health/BP_HealthComponent` (`self.GetComponentByClass` OtherActor "/Game/Health/BP_HealthComponent.BP_HealthComponent_C")))
    (set `self.bImpactProcessed` true)
    (`/Game/Health/BP_HealthComponent.TakeDamage` _asbp_health_component (`self.DamageAmount`))
    (`self.K2_DestroyActor` self)))

(fn `UserConstructionScript`)