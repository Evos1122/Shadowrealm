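; Test enemy that chases the player character and deals periodic melee damage while alive.
; Tick checks its own HealthComponent and the distance to player 0, chasing within detection range through SimpleMoveToActor and stopping when dead, out of range or in attack range.
; In attack range, an accumulated delta-time cooldown triggers TakeDamage on the player's BP_HealthComponent.
; A disconnected duplicate of this logic never runs.
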(event `self.ReceiveTick`
  (params (DeltaSeconds :type "Float (single-precision)"))
  (bind _returnvalue (`self.GetController`))
  (bind _returnvalue_2 (`GameplayStatics.GetPlayerCharacter` 0))
  (bind _returnvalue_3 (`self.GetDistanceTo` self _returnvalue_2))
  (`/Engine/EditorBlueprintResources/StandardMacros.IsValid` _returnvalue_2
    (:`Is Valid`
      (bind _dead (`/Game/Health/BP_HealthComponent.IsDead` (`self.HealthComponent`)))
      (if _dead
        (`Controller.StopMovement` _returnvalue)
        (set `self.AttackCooldown` 0.0)
        (elif (<= _returnvalue_3 1200.0)
          (if (> _returnvalue_3 160.0)
            (`AIBlueprintHelperLibrary.SimpleMoveToActor` _returnvalue _returnvalue_2)
            (set `self.AttackCooldown` 0.0)
            (else
              (`Controller.StopMovement` _returnvalue)
              (set `self.AttackCooldown` (+ (`self.AttackCooldown`) DeltaSeconds))
              (if (>= (`self.AttackCooldown`) 1.0)
                (bind _asbp_health_component (cast `/Game/Health/BP_HealthComponent` (`self.GetComponentByClass` _returnvalue_2 "/Game/Health/BP_HealthComponent.BP_HealthComponent_C")))
                (`/Game/Health/BP_HealthComponent.TakeDamage` _asbp_health_component 25.0)
                (set `self.AttackCooldown` 0.0))))
          (else
            (`Controller.StopMovement` _returnvalue)
            (set `self.AttackCooldown` 0.0)))))
    (:`Is Not Valid`
      (set `self.AttackCooldown` 0.0))))

(fn `UserConstructionScript`)